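; BP_Kniha is a book pickup (kniha is Czech for book) that opens a UI widget when picked up.
; On pickup, Otevri creates WB_Kniha, adds it to the viewport, hides the Cube, disables its collision and sets the Picked flag.
; On close, Zavreno removes the widget, restores the Cube's visibility and collision, and clears the flag.
; The Otevreno function and construction script are empty.
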(event Custom|Zavreno
  (Widget|RemovefromParent (stale Custom|Otevri _returnvalue))
  (Rendering|SetVisibility (Variables|Default|GetCube) true false)
  (Collision|SetCollisionEnabled (Variables|Default|GetCube) "QueryAndPhysics")
  (Variables|Default|Setpicked false))

(event Custom|Otevri
  (bind _returnvalue (UserInterface|CreateWidget "/Game/mojeBlueprinty/WB_Kniha.WB_Kniha_C"))
  (UserInterface|Viewport|AddtoViewport _returnvalue 0)
  (Rendering|SetVisibility (Variables|Default|GetCube) false false)
  (Collision|SetCollisionEnabled (Variables|Default|GetCube) "NoCollision")
  (Variables|Default|Setpicked true))

(event EventEventonPickup
  (CallFunction|Otevri))

(event EventEventonClose
  (CallFunction|Zavreno))

(fn ConstructionScript)

(fn Otevreno)